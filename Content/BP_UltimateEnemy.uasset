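; BP_UltimateEnemy is an enemy Blueprint that traces the events of its AI controller's utility AI component.
; On BeginPlay it casts its controller to UltimateAIController and binds handlers for action changed, not available, spawned and initialized, printing a warning if the cast fails.
; Each handler only prints a red debug message, with the action names where provided.
; Chosen, ticked and before-score-computation handlers exist, but their bindings are disconnected and never run.
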(event Custom|OnUtilityAIActionChanged
  (params (NewAction :type Utility%20AI%20Action%20Object%20Reference) (OldAction :type Utility%20AI%20Action%20Object%20Reference))
  (Development|PrintString (Utilities|String|Append "OnUtilityAIActionChanged , old: " (Utilities|GetDisplayName OldAction) ", new: " (Utilities|GetDisplayName NewAction)) true true "(R=1.000000,G=0.000000,B=0.000000,A=1.000000)" 5.0))

(event Custom|OnUtilityAIActionChoosen
  (params (Action :type Utility%20AI%20Action%20Object%20Reference))
  (Development|PrintString (Utilities|String|Append "OnUtilityAIActionChoosen for " (Utilities|GetDisplayName Action)) true true "(R=1.000000,G=0.000000,B=0.000000,A=1.000000)" 5.0))

(event Custom|OnUtilityAIActionNotAvailable
  (Development|PrintString "OnUtilityAIActionNotAvailable" true true "(R=1.000000,G=0.000000,B=0.000000,A=1.000000)" 5.0))

(event Custom|OnUtilityAIActionSpawned
  (params (Action :type Utility%20AI%20Action%20Object%20Reference))
  (Development|PrintString (Utilities|String|Append "OnUtilityAIActionSpawned for " (Utilities|GetDisplayName Action)) true true "(R=1.000000,G=0.000000,B=0.000000,A=1.000000)" 5.0))

(event Custom|OnUtilityAIActionTicked
  (params (Action :type Utility%20AI%20Action%20Object%20Reference))
  (Development|PrintString (Utilities|String|Append "OnUtilityAIActionTicked for " (Utilities|GetDisplayName Action)) true true "(R=1.000000,G=0.000000,B=0.000000,A=1.000000)" 5.0))

(event Custom|OnUtilityAIBeforeScoreComputation
  (Development|PrintString "OnUtilityAIBeforeScoreComputation" true true "(R=1.000000,G=0.000000,B=0.000000,A=1.000000)" 5.0))

(event Custom|OnUtilityAiInitialized
  (Development|PrintString "OnUtilityAiInitialized" true true "(R=1.000000,G=0.000000,B=0.000000,A=1.000000)" 5.0))

(event EventBeginPlay
  (bind _asultimate_aicontroller (Utilities|Casting|CastToUltimateAIController (Pawn|GetController))
    (:then
      (EventDispatchers|AssignOnUtilityAIActionChanged (Class|UltimateAIController|GetUtilityAIComponent _asultimate_aicontroller) (delegate Custom|OnUtilityAIActionChanged))
      (EventDispatchers|AssignOnUtilityAIActionNotAvailable (Class|UltimateAIController|GetUtilityAIComponent _asultimate_aicontroller) (delegate Custom|OnUtilityAIActionNotAvailable))
      (EventDispatchers|AssignOnUtilityAIActionSpawned (Class|UltimateAIController|GetUtilityAIComponent _asultimate_aicontroller) (delegate Custom|OnUtilityAIActionSpawned))
      (EventDispatchers|AssignOnUtilityAIInitialized (Class|UltimateAIController|GetUtilityAIComponent _asultimate_aicontroller) (delegate Custom|OnUtilityAiInitialized)))
    (:CastFailed
      (Development|PrintString "Invalid ai controller type"))))

(fn ConstructionScript)